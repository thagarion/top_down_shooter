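; BP_Ammo_Crate is an ammo crate Blueprint that shows weapon details on its pickup widget.
; On BeginPlay, after the parent logic, it casts the PickUpWidget component's widget to PickUpWeapon_Widget.
; It then fills in the name, bullet count and icon from GetWeaponInfo, using the maximum projectile count as the bullet count.
; Tick is disabled, and the construction script only calls the parent.
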(event `self.ReceiveBeginPlay`
  (`parent.ReceiveBeginPlay`)
  (bind _aspick_up_weapon_widget (cast `/Game/Blueprints/Widgets/PickUpWeapon_Widget` (`WidgetComponent.GetWidget` (`self.Pick Up Widget`))))
  (bind _returnvalue (`self.GetWeaponInfo`))
  (`/Game/Blueprints/Widgets/PickUpWeapon_Widget.SetWeaponName` _aspick_up_weapon_widget (break `WeaponInfo` _returnvalue))
  (`/Game/Blueprints/Widgets/PickUpWeapon_Widget.SetBulletCount` _aspick_up_weapon_widget (`.MaxProjectileCount` (break `WeaponInfo` _returnvalue)))
  (`/Game/Blueprints/Widgets/PickUpWeapon_Widget.SetWeaponIcon` _aspick_up_weapon_widget (`.WeaponIcon` (break `WeaponInfo` _returnvalue))))

(fn `UserConstructionScript`
  (`parent.UserConstructionScript`))