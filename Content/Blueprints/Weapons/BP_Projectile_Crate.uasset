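; BP_Projectile_Crate is a weapon ammo crate that shows what it holds on a pickup widget.
; On BeginPlay it runs the parent logic, then casts its PickUpWidget component's widget to PickUpAmmo_Widget.
; It fills that widget with the weapon name and icon from GetWeaponInfo and the stored projectile count from GetWeaponStats.
; The widget is set only at BeginPlay, and the graphs here add no other behavior to the parent.
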(event `self.ReceiveBeginPlay`
  (`parent.ReceiveBeginPlay`)
  (bind _aspick_up_ammo_widget (cast `/Game/Blueprints/Widgets/PickUpAmmo_Widget` (`WidgetComponent.GetWidget` (`self.Pick Up Widget`))))
  (bind _returnvalue (`self.GetWeaponInfo`))
  (`/Game/Blueprints/Widgets/PickUpAmmo_Widget.SetWeaponName` _aspick_up_ammo_widget (break `WeaponInfo` _returnvalue))
  (`/Game/Blueprints/Widgets/PickUpAmmo_Widget.SetWeaponIcon` _aspick_up_ammo_widget (`.WeaponIcon` (break `WeaponInfo` _returnvalue)))
  (bind _returnvalue_2 (`self.GetWeaponStats`))
  (`/Game/Blueprints/Widgets/PickUpAmmo_Widget.SetBulletCount` _aspick_up_ammo_widget (`.StoredProjectileCount` (break `WeaponStats` _returnvalue_2))))

(fn `UserConstructionScript`
  (`parent.UserConstructionScript`))