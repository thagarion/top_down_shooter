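; BP_Weapon_Item is a weapon item actor that fills in its pickup widget with the weapon's details.
; On BeginPlay it runs the parent logic, then casts its WidgetComponent's widget to BPW_PickUpWeapon.
; It passes the name, maximum projectile count (shown as bullet count) and icon from GetWeaponInfo to that widget once, with no Tick logic.
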(event `self.ReceiveBeginPlay`
  (`parent.ReceiveBeginPlay`)
  (bind _aspick_up_weapon_widget (cast `/Game/Blueprints/Widgets/BPW_PickUpWeapon` (`WidgetComponent.GetWidget` (`self.WidgetComponent`))))
  (bind _returnvalue (`self.GetWeaponInfo`))
  (`/Game/Blueprints/Widgets/BPW_PickUpWeapon.SetWeaponName` _aspick_up_weapon_widget (break `WeaponInfo` _returnvalue))
  (`/Game/Blueprints/Widgets/BPW_PickUpWeapon.SetBulletCount` _aspick_up_weapon_widget (`.MaxProjectileCount` (break `WeaponInfo` _returnvalue)))
  (`/Game/Blueprints/Widgets/BPW_PickUpWeapon.SetWeaponIcon` _aspick_up_weapon_widget (`.WeaponIcon` (break `WeaponInfo` _returnvalue))))

(fn `UserConstructionScript`
  (`parent.UserConstructionScript`))