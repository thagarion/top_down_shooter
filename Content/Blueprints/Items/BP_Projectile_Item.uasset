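; BP_Projectile_Item is an item Blueprint that shows weapon and ammo details on a pickup widget.
; On BeginPlay it runs the parent logic, then casts its WidgetComponent's widget to BPW_PickUpAmmo.
; It fills the widget once with name and icon from GetWeaponInfo and the stored projectile count from GetWeaponStats.
; The construction script only calls the parent.
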(event `self.ReceiveBeginPlay`
  (`parent.ReceiveBeginPlay`)
  (bind _aspick_up_ammo_widget (cast `/Game/Blueprints/Widgets/BPW_PickUpAmmo` (`WidgetComponent.GetWidget` (`self.WidgetComponent`))))
  (bind _returnvalue (`self.GetWeaponInfo`))
  (`/Game/Blueprints/Widgets/BPW_PickUpAmmo.SetWeaponName` _aspick_up_ammo_widget (break `WeaponInfo` _returnvalue))
  (`/Game/Blueprints/Widgets/BPW_PickUpAmmo.SetWeaponIcon` _aspick_up_ammo_widget (`.WeaponIcon` (break `WeaponInfo` _returnvalue)))
  (bind _returnvalue_2 (`self.GetWeaponStats`))
  (`/Game/Blueprints/Widgets/BPW_PickUpAmmo.SetBulletCount` _aspick_up_ammo_widget (`.StoredProjectileCount` (break `WeaponStats` _returnvalue_2))))

(fn `UserConstructionScript`
  (`parent.UserConstructionScript`))