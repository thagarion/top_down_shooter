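; Top-down character Blueprint that adds damage feedback, firing animation and camera shake to inherited weapon logic.
; HealthComponent damage spawns separate shield and health damage-number widgets at the capsule's screen position, while death plays a death montage.
; Fire input, blocked while reloading, forwards to the fire functions and picks an ironsights or hip montage by movement state.
; J, H and V keys trigger random projectile drop, random weapon drop and the death montage.
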(event `self.HealthComponent.OnTakeDamage`
  (params (HealthDamage :type "Float (single-precision)") (ShieldDamage :type "Float (single-precision)"))
  (bind _returnvalue (- (`GameplayStatics.ProjectWorldToScreen` (`GameplayStatics.GetPlayerController` 0) (`SceneComponent.K2_GetComponentLocation` (`self.CapsuleComponent`))) (64.0 16.0)))
  (if (> ShieldDamage 0.0)
    (bind _returnvalue_2 (`|CreateWidget` "/Game/Blueprints/Widgets/DamagNumber_Widget.DamagNumber_Widget_C" null _returnvalue ShieldDamage true))
    (`UserWidget.AddToViewport` _returnvalue_2 0))
  (if (> HealthDamage 0.0)
    (bind _returnvalue_3 (`|CreateWidget` "/Game/Blueprints/Widgets/DamagNumber_Widget.DamagNumber_Widget_C" null _returnvalue HealthDamage))
    (`UserWidget.AddToViewport` _returnvalue_3 0)))

(event `Key|J`
  (params (Key :type "Key Structure"))
  (:`Pressed`
    (`self.DropRandomProjectile`)))

(event `Key|H`
  (params (Key :type "Key Structure"))
  (:`Pressed`
    (`self.DropRandomWeapon`)))

(event `Key|V`
  (params (Key :type "Key Structure"))
  (:`Pressed`
    (`|PlayMontage` (`self.Mesh`) "/Game/Blueprints/Character/Mannequin/Animations/ThirdPerson_Death_1_Montage.ThirdPerson_Death_1_Montage" :!label _label)))

(event `self.HealthComponent.OnDead`
  (goto _label))

(event `InputAction|Fire`
  (params (Key :type "Key Structure"))
  (bind _mesh (`self.Mesh`))
  (:`Pressed`
    (bind _returnvalue (`self.GetIsReloading`))
    (if (not _returnvalue)
      (`self.FireButtonPressed`)
      (if (`|EnumEquality` "AIM_State" (`self.MovementState`))
        (`|PlayMontage` _mesh "/Game/Blueprints/Character/Mannequin/Animations/ThirdPerson_Fire_Rifle_Ironsights_Montage.ThirdPerson_Fire_Rifle_Ironsights_Montage")
        (else
          (`|PlayMontage` _mesh "/Game/Blueprints/Character/Mannequin/Animations/ThirdPerson_Fire_Rifle_Hip_Montage.ThirdPerson_Fire_Rifle_Hip_Montage")))))
  (:`Released`
    (`self.FireButtonReleased`)))

(fn `CameraShakeEvent`
  (`GameplayStatics.PlayWorldCameraShake` "/Game/Blueprints/Game/BP_CameraShake.BP_CameraShake_C" (`SceneComponent.K2_GetComponentLocation` (`self.TopDownCameraComponent`)) 0.0 30.0))

(fn `GetCursorToWorld`
  (returns (ReturnValue :type "DecalComponent Object Reference"))
  (return null))

(fn `UserConstructionScript`)