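; BP_Zombie is a zombie character Blueprint that shows combat feedback driven by its HealthComponent.
; Damage and heal events each spawn a floating number widget at the capsule's projected screen position, nudged slightly upward.
; On BeginPlay it binds the health component to its health bar widget component, and the component's death event calls Die.
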(event `self.HealthComponent.OnTakeDamage`
  (params (Damage :type "Float (single-precision)"))
  (bind _returnvalue (`|CreateWidget` "/Game/Blueprints/Widgets/BPW_DamageNumber.BPW_DamageNumber_C" null (- (`GameplayStatics.ProjectWorldToScreen` (`GameplayStatics.GetPlayerController` 0) (`SceneComponent.K2_GetComponentLocation` (`self.CapsuleComponent`))) (0.0 16.0)) Damage))
  (`UserWidget.AddToViewport` _returnvalue 0))

(event `self.HealthComponent.OnTakeHeal`
  (params (Value :type "Float (single-precision)"))
  (bind _returnvalue (`|CreateWidget` "/Game/Blueprints/Widgets/BPW_HealNumber.BPW_HealNumber_C" null (- (`GameplayStatics.ProjectWorldToScreen` (`GameplayStatics.GetPlayerController` 0) (`SceneComponent.K2_GetComponentLocation` (`self.CapsuleComponent`))) (0.0 16.0)) Value))
  (`UserWidget.AddToViewport` _returnvalue 0))

(event `self.ReceiveBeginPlay`
  (bind _asbpw_health_bar (cast `/Game/Blueprints/Widgets/BPW_HealthBar` (`WidgetComponent.GetWidget` (`self.HealthBarWidgetComponent`))))
  (`/Game/Blueprints/Widgets/BPW_HealthBar.SetHealthComponent` _asbpw_health_bar (`self.HealthComponent`)))

(event `self.HealthComponent.OnDead`
  (`self.Die`))

(fn `UserConstructionScript`)